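; BP_Weapon is the player's melee weapon actor, which attaches itself to the Weapon socket on the BP_Seeker pawn's mesh at BeginPlay.
; Its box overlap registers hits only while the Seeker's IsAttacking flag is set, ignoring the player's own pawn.
; A hit plays a sound at the other actor's location and prints its name; no damage is applied here.
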(event `self.ReceiveBeginPlay`
  (bind _asbp_seeker (cast `/Game/FirstPersonBP/BP_Seeker` (`GameplayStatics.GetPlayerPawn` 0)))
  (`self.K2_AttachToComponent` (`Character.Mesh` _asbp_seeker) "Weapon" "SnapToTarget" "SnapToTarget" "SnapToTarget"))

(event `self.Box.OnComponentBeginOverlap`
  (params (OverlappedComponent :type "PrimitiveComponent Object Reference") (OtherActor :type "Actor Object Reference") (OtherComp :type "PrimitiveComponent Object Reference") (OtherBodyIndex :type Integer) (bFromSweep :type Boolean) (SweepResult :type "HitResult Structure (by ref)"))
  (bind _returnvalue (`GameplayStatics.GetPlayerPawn` 0))
  ;[1 1 1] Hit animations
  (bind _asbp_seeker (cast `/Game/FirstPersonBP/BP_Seeker` _returnvalue))
  (if (and (`/Game/FirstPersonBP/BP_Seeker.isAttacking?` _asbp_seeker) (!= OtherActor _returnvalue))
    (`GameplayStatics.PlaySoundAtLocation` "/Game/Character/Hit_Sound.Hit_Sound" (`self.K2_GetActorLocation` OtherActor))
    (`KismetSystemLibrary.PrintString` (`KismetSystemLibrary.GetDisplayName` OtherActor))))

(fn `UserConstructionScript`)