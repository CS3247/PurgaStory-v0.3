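; Multiplayer Game State for a one-Seeker, one-Hider match, running the flow from waiting screen through hiding and chase phases to game end.
; BeginPlay caches both characters and randomly picks inner and outer post-process colors.
; When all players are ready, a self-calling one-second countdown releases the Seeker, then an authority-only chase countdown reuses HidingTimer.
; WinRequest accepts only the first winner and triggers each character's win or loss.
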(event `self.ReceiveTick`
  (params (DeltaSeconds :type "Float (single-precision)"))
  ;[1 1 1] Event Tick
)

(event `CheckAllPlayersReady`
  ;[1 1 1] Checks if all players are ready and starts the game when they are
  (for _array_element (`self.PlayerArray`)
    (`KismetSystemLibrary.PrintString` "START LOOP")
    (bind _asps_mp (cast `/Game/Multiplayer/Blueprints/PS_MP` _array_element))
    (bind _isready (`/Game/Multiplayer/Blueprints/PS_MP.isReady` _asps_mp))
    (`KismetSystemLibrary.PrintString` (`KismetStringLibrary.Concat_StrStr` (`KismetStringLibrary.Conv_IntToString` (`PlayerState.PlayerId` _array_element)) (`KismetStringLibrary.Conv_BoolToString` _isready)))
    (if _isready
      (set `self.isAllPlayersReady` true)
      (else
        (set `self.isAllPlayersReady` false)
        (break))))
  (`KismetSystemLibrary.PrintString` "COMPLETED")
  (if (`self.isAllPlayersReady`)
    (`KismetSystemLibrary.PrintString` "TRUE")
    (`self.PreGameStart`)))

(event `GetActorReference`
  ;[1 1 1] Get Actor References Event
  (bind _outactors (`GameplayStatics.GetAllActorsOfClass` "/Game/FirstPersonBP/BP_Seeker.BP_Seeker_C"))
  (set `self.SeekerRef` (`KismetArrayLibrary.Array_Get` _outactors))
  (bind _outactors_2 (`GameplayStatics.GetAllActorsOfClass` "/Game/ThirdPersonBP/BP_Hider.BP_Hider_C"))
  (set `self.HiderRef` (`KismetArrayLibrary.Array_Get` _outactors_2)))

(event `self.ReceiveBeginPlay`
  ;[1 1 1] Waiting Screen
  (`self.GetActorReference`)
  (`self.ResetVariables`)
  (`self.choosePostProcess`)
  (`/Game/ThirdPersonBP/BP_Hider.CreateWaitingScreen` (`self.HiderRef`))
  (`/Game/FirstPersonBP/BP_Seeker.CreateWaitingScreen` (`self.SeekerRef`)))

(event `ResetVariables`
  ;[1 1 1] Reset Variables Event
  (set `self.isGameOver` false)
  (set `self.isSeekerReady` false)
  (set `self.isHiderReady` false)
  (set `self.HidingTimer` (`self.HidingTimerDefaultValue`)))

(event `PreGameStart`
  (bind _seekerref (`self.SeekerRef`))
  (bind _hiderref (`self.HiderRef`))
  ;[1 1 1] Pre-game Setup
  (`/Game/ThirdPersonBP/BP_Hider.RemoveWaitingScreen` _hiderref)
  (set `/Game/ThirdPersonBP/BP_Hider.canMove` true _hiderref)
  (`/Game/ThirdPersonBP/BP_Hider.CreateChaseUI` _hiderref)
  (`/Game/FirstPersonBP/BP_Seeker.RemoveWaitingScreen` _seekerref)
  (`/Game/FirstPersonBP/BP_Seeker.CreateReaperTimer` _seekerref)
  (set `self.HidingTimer` (`self.HidingTimerDefaultValue`))
  (`self.CountdownAndRemoveHiderTimer`))

(event `RunHiderTimer`
  ;[1 1 1] Hiding Timer
  (`/Game/ThirdPersonBP/BP_Hider.CreateHidingTimerWidget` (`self.HiderRef`))
  (`/Game/FirstPersonBP/BP_Seeker.CreateHidingTimerWidget` (`self.SeekerRef`))
  (`self.CountdownAndRemoveHiderTimer`))

(event `RunChaseTimer`
  (`/Engine/EditorBlueprintResources/ActorMacros.Switch Has Authority`
    (:`Authority`
      (`self.CountdownAndRemoveChaseTimer`))))

(event `InitialiseTimerToChaseTime`
  (set `self.HidingTimer` (`self.ChaseTimerDefaultValue`)))

(event `CountdownAndRemoveHiderTimer`
  ;[1 1 1] Hiding Timer
  (if (<= (`self.HidingTimer`) 0)
    (`self.ChaseStart`)
    (else
      (`KismetSystemLibrary.Delay` 1.0)
      (`self.DecrementHidingTimer`)
      (`self.CountdownAndRemoveHiderTimer`))))

(event `CountdownAndRemoveChaseTimer`
  (`/Engine/EditorBlueprintResources/ActorMacros.Switch Has Authority`
    (:`Authority`
      (if (not (<= (`self.HidingTimer`) 0))
        (`KismetSystemLibrary.Delay` 1.0)
        (`self.DecrementHidingTimer`)
        (`self.CountdownAndRemoveChaseTimer`)))))

(event `ChaseStart`
  (bind _seekerref (`self.SeekerRef`))
  ;[1 1 1] Chase Start
  (`/Game/FirstPersonBP/BP_Seeker.RemoveReaperTimer` _seekerref)
  (`/Game/FirstPersonBP/BP_Seeker.CreateChaseUI` _seekerref)
  (`/Game/FirstPersonBP/BP_Seeker.SetInitialSkillCooldown` _seekerref)
  (set `/Game/FirstPersonBP/BP_Seeker.canMove` true _seekerref)
  (set `self.HidingTimer` (`self.ChaseTimerDefaultValue`))
  (set `self.isChasePhase` true)
  (`self.RunChaseTimer`))

(event `WinRequest`
  (params (winnerID :type Integer))
  (if (not (`self.isGameOver`))
    (set `self.isGameOver` true)
    (set `self.winID` winnerID)
    (`self.GameEnd`)))

(event `GameEnd`
  (bind _winid (`self.winID`))
  (bind _hiderref (`self.HiderRef`))
  (bind _seekerref (`self.SeekerRef`))
  (`WidgetLayoutLibrary.RemoveAllWidgets`)
  (if (== _winid (`self.DefaultSeekerPlayerID`))
    (`/Game/FirstPersonBP/BP_Seeker.seeker_win` _seekerref)
    (`/Game/ThirdPersonBP/BP_Hider.hider_death` _hiderref)
    (`/Game/ThirdPersonBP/BP_Hider.server_hider_death` _hiderref)
    (elif (== _winid (`self.DefaultHiderPlayerID`))
      (`/Game/FirstPersonBP/BP_Seeker.seeker_lose` _seekerref)
      (`/Game/FirstPersonBP/BP_Seeker.seeker_lose_client` _seekerref)
      (`/Game/ThirdPersonBP/BP_Hider.hider_win` _hiderref))))

(event `choosePostProcess`
  (switch `int` (`KismetMathLibrary.RandomIntegerInRange` 0 2)
    (:`0`
      (set `self.ppv OUT chosen` (`self.ppv out red`)))
    (:`1`
      (set `self.ppv OUT chosen` (`self.ppv out green`)))
    (:`2`
      (set `self.ppv OUT chosen` (`self.ppv out blue`))))
  (switch `int` (`KismetMathLibrary.RandomIntegerInRange` 0 2)
    (:`0`
      (set `self.ppv IN chosen` (`self.ppv in red`)))
    (:`1`
      (set `self.ppv IN chosen` (`self.ppv in green`)))
    (:`2`
      (set `self.ppv IN chosen` (`self.ppv in blue`)))))

(fn `DecrementHidingTimer`
  (set `self.HidingTimer` (- (`self.HidingTimer`) 1)))

(fn `OnRep_HidingTimer`)

(fn `OnRep_isHiderReady`)

(fn `OnRep_isSeekerReady`)

(fn `OnRep_ppv IN chosen`)

(fn `OnRep_ppv OUT chosen`)

(fn `Test`
  (bind _ishiderready (`self.isHiderReady`))
  (if (`self.isSeekerReady`)
    (`KismetSystemLibrary.PrintString` "SeekerReady")
    (if _ishiderready
      (`KismetSystemLibrary.PrintString` "HiderReady" :!label _label)
      (else
        (`KismetSystemLibrary.PrintString` "HiderWAITING" :!label _label_2)))
    (else
      (`KismetSystemLibrary.PrintString` "SeekerWAITING")
      (if _ishiderready
        (goto _label)
        (else
          (goto _label_2))))))

(fn `UserConstructionScript`)